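; BP_TargetActorTest is a test target actor that displays a health and mana bar widget in the world.
; On BeginPlay it initializes the WBP_HealthMana widget with its ASC.
; Every tick, WidgetLookAtCamera turns the widget component toward player 0's camera on yaw only, zeroing pitch and roll so the display stays upright.
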(event `self.ReceiveBeginPlay`
  (bind _aswbp_health_mana (cast `/Game/Blueprints/UI/WBP_HealthMana` (`WidgetComponent.GetUserWidgetObject` (`self.Health Mana Widget`))))
  (`/Game/Blueprints/UI/WBP_HealthMana.Init` _aswbp_health_mana (`self.ASC`)))

(event `self.ReceiveTick`
  (params (DeltaSeconds :type "Float (single-precision)"))
  (`self.WidgetLookAtCamera` (`self.Health Mana Widget`)))

(fn `UserConstructionScript`)

(fn `WidgetLookAtCamera`
  (params (InWidget :type "WidgetComponent Object Reference"))
  (bind (_returnvalue_roll _returnvalue_pitch _returnvalue_yaw) (`KismetMathLibrary.BreakRotator` (`KismetMathLibrary.FindLookAtRotation` (`SceneComponent.K2_GetComponentLocation` InWidget) (`PlayerCameraManager.GetCameraLocation` (`GameplayStatics.GetPlayerCameraManager` 0)))))
  (`SceneComponent.K2_SetWorldRotation` InWidget (`KismetMathLibrary.MakeRotator` 0.0 0.0 _returnvalue_yaw) false false))